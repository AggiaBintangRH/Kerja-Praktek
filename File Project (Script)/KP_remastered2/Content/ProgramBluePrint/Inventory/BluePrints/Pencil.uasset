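; Pencil pickup actor that goes into the player's inventory as item 5 and completes an objective.
; It becomes collectible after a short delay from BeginPlay; any box overlap then checks the player character's eight slot variables through nested branches.
; The first empty slot receives the item, then the actor destroys itself, sets HasKey5 and shows the ObjectiveComplete widget.
; When all slots are occupied, it shows the InventoryFull widget instead.
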(event OnComponentBeginOverlap(Box)
  (params (OverlappedComponent :type Primitive%20Component%20Object%20Reference) (OtherActor :type Actor%20Object%20Reference) (OtherComp :type Primitive%20Component%20Object%20Reference) (OtherBodyIndex :type Integer) (bFromSweep :type Boolean) (SweepResult :type Hit%20Result%20Structure%20%28by%20ref%29))
  (if (Variables|Default|GetCanPickUp)
    (bind _asthird_person_character (Utilities|Casting|CastToThirdPersonCharacter (Game|GetPlayerCharacter 0)))
    (if (== (Variables|/Game/ProgramBluePrint/Player/Player/ThirdPersonCharacter.ThirdPersonCharacter_C|GetSlot1Item _asthird_person_character) 0)
      (Variables|/Game/ProgramBluePrint/Player/Player/ThirdPersonCharacter.ThirdPersonCharacter_C|SetSlot1Item _asthird_person_character 5)
      (Actor|DestroyActor :!label _label)
      (bind _asthird_person_character_2 (Utilities|Casting|CastToThirdPersonCharacter (Game|GetPlayerCharacter 0)))
      (Variables|/Game/ProgramBluePrint/Player/Player/ThirdPersonCharacter.ThirdPersonCharacter_C|SetHasKey5 _asthird_person_character_2 true)
      (bind _returnvalue (UserInterface|CreateWidget "/Game/ProgramBluePrint/PlayerObjective/Widget/ObjectiveComplete.ObjectiveComplete_C"))
      (UserInterface|Viewport|AddtoViewport _returnvalue 0)
      (elif (== (Variables|/Game/ProgramBluePrint/Player/Player/ThirdPersonCharacter.ThirdPersonCharacter_C|GetSlot2Item _asthird_person_character) 0)
        (Variables|/Game/ProgramBluePrint/Player/Player/ThirdPersonCharacter.ThirdPersonCharacter_C|SetSlot2Item _asthird_person_character 5)
        (goto _label)
        (elif (== (Variables|/Game/ProgramBluePrint/Player/Player/ThirdPersonCharacter.ThirdPersonCharacter_C|GetSlot3Item _asthird_person_character) 0)
          (Variables|/Game/ProgramBluePrint/Player/Player/ThirdPersonCharacter.ThirdPersonCharacter_C|SetSlot3Item _asthird_person_character 5)
          (goto _label)
          (elif (== (Variables|/Game/ProgramBluePrint/Player/Player/ThirdPersonCharacter.ThirdPersonCharacter_C|GetSlot4Item _asthird_person_character) 0)
            (Variables|/Game/ProgramBluePrint/Player/Player/ThirdPersonCharacter.ThirdPersonCharacter_C|SetSlot4Item _asthird_person_character 5)
            (goto _label)
            (elif (== (Variables|/Game/ProgramBluePrint/Player/Player/ThirdPersonCharacter.ThirdPersonCharacter_C|GetSlot5Item _asthird_person_character) 0)
              (Variables|/Game/ProgramBluePrint/Player/Player/ThirdPersonCharacter.ThirdPersonCharacter_C|SetSlot5Item _asthird_person_character 5)
              (goto _label)
              (elif (== (Variables|/Game/ProgramBluePrint/Player/Player/ThirdPersonCharacter.ThirdPersonCharacter_C|GetSlotItem6 _asthird_person_character) 0)
                (Variables|/Game/ProgramBluePrint/Player/Player/ThirdPersonCharacter.ThirdPersonCharacter_C|SetSlotItem6 _asthird_person_character 5)
                (goto _label)
                (elif (== (Variables|/Game/ProgramBluePrint/Player/Player/ThirdPersonCharacter.ThirdPersonCharacter_C|GetSlotItem7 _asthird_person_character) 0)
                  (Variables|/Game/ProgramBluePrint/Player/Player/ThirdPersonCharacter.ThirdPersonCharacter_C|SetSlotItem7 _asthird_person_character 5)
                  (goto _label)
                  (elif (== (Variables|/Game/ProgramBluePrint/Player/Player/ThirdPersonCharacter.ThirdPersonCharacter_C|GetSlotItem8 _asthird_person_character) 0)
                    (Variables|/Game/ProgramBluePrint/Player/Player/ThirdPersonCharacter.ThirdPersonCharacter_C|SetSlotItem8 _asthird_person_character 5)
                    (goto _label)
                    (else
                      (bind _returnvalue_2 (UserInterface|CreateWidget "/Game/ProgramBluePrint/Inventory/Widget/InventoryFull.InventoryFull_C"))
                      (UserInterface|Viewport|AddtoViewport _returnvalue_2 0))))))))))))

(event EventBeginPlay
  (Utilities|FlowControl|Delay 3.0)
  (Variables|Default|SetCanPickUp true))

(fn ConstructionScript)