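; Jacket pickup that, three seconds after BeginPlay, can be collected by player overlap to advance the objective.
; It puts item 1 in the first empty of eight character inventory slots, or shows an InventoryFull widget.
; On pickup it destroys itself, sets HasKey1 and shows ObjectiveComplete.
; The objective becomes "Talk To Administrator", or "Go To FTI" if Pencil is set, and is written to the SaveGameObject slot.
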(event OnComponentBeginOverlap(Box)
  (params (OverlappedComponent :type Primitive%20Component%20Object%20Reference) (OtherActor :type Actor%20Object%20Reference) (OtherComp :type Primitive%20Component%20Object%20Reference) (OtherBodyIndex :type Integer) (bFromSweep :type Boolean) (SweepResult :type Hit%20Result%20Structure%20%28by%20ref%29))
  (if (Variables|Default|GetCanPickUp)
    (bind _asthird_person_character (Utilities|Casting|CastToThirdPersonCharacter (Game|GetPlayerCharacter 0)))
    (if (== (Variables|/Game/ProgramBluePrint/Player/Player/ThirdPersonCharacter.ThirdPersonCharacter_C|GetSlot1Item _asthird_person_character) 0)
      (Variables|/Game/ProgramBluePrint/Player/Player/ThirdPersonCharacter.ThirdPersonCharacter_C|SetSlot1Item _asthird_person_character 1)
      (Actor|DestroyActor :!label _label)
      (bind _asthird_person_character_2 (Utilities|Casting|CastToThirdPersonCharacter (Game|GetPlayerCharacter 0)))
      (Utilities|FlowControl|Sequence
        (:then_0
          (Variables|/Game/ProgramBluePrint/Player/Player/ThirdPersonCharacter.ThirdPersonCharacter_C|SetHasKey1 _asthird_person_character_2 true)
          (bind _returnvalue (UserInterface|CreateWidget "/Game/ProgramBluePrint/PlayerObjective/Widget/ObjectiveComplete.ObjectiveComplete_C"))
          (UserInterface|Viewport|AddtoViewport _returnvalue 0)
          (bind _asthird_person_character_3 (Utilities|Casting|CastToThirdPersonCharacter (Game|GetPlayerCharacter 0)))
          (Variables|/Game/ProgramBluePrint/Player/Player/ThirdPersonCharacter.ThirdPersonCharacter_C|SetPlayerObjective _asthird_person_character_3 "Talk To Administrator")
          (bind _returnvalue_2 (SaveGame|DoesSaveGameExist "SaveGameObject"))
          (if _returnvalue_2
            (bind _returnvalue_3 (SaveGame|LoadGamefromSlot "SaveGameObject"))
            (bind _output_get (Variables|Default|SetSaverSubClass _returnvalue_3))
            (bind _assave_game_object (Utilities|Casting|CastToSaveGameObject _output_get))
            (Variables|/Game/ProgramBluePrint/PlayerObjective/SaveObjective/SaveGameObject.SaveGameObject_C|SetPlayerObjective _assave_game_object "Talk To Administrator")
            (SaveGame|SaveGametoSlot (Variables|Default|GetSaverSubClass) "SaveGameObject")
            (else
              (bind _returnvalue_4 (SaveGame|CreateSaveGameObject "/Game/ProgramBluePrint/PlayerObjective/SaveObjective/SaveGameObject.SaveGameObject_C"))
              (bind _output_get_2 (Variables|Default|SetSaverSubClass _returnvalue_4))
              (bind _assave_game_object_2 (Utilities|Casting|CastToSaveGameObject _output_get_2))
              (Variables|/Game/ProgramBluePrint/PlayerObjective/SaveObjective/SaveGameObject.SaveGameObject_C|SetPlayerObjective _assave_game_object_2 "Talk To Administrator")
              (SaveGame|SaveGametoSlot (Variables|Default|GetSaverSubClass) "SaveGameObject"))))
        (:then_1
          (if (Variables|/Game/ProgramBluePrint/Player/Player/ThirdPersonCharacter.ThirdPersonCharacter_C|GetPencil _asthird_person_character_2)
            (Variables|/Game/ProgramBluePrint/Player/Player/ThirdPersonCharacter.ThirdPersonCharacter_C|SetPlayerObjective _asthird_person_character_2 "Go To FTI")
            (bind _returnvalue_5 (SaveGame|DoesSaveGameExist "SaveGameObject"))
            (if _returnvalue_5
              (bind _returnvalue_6 (SaveGame|LoadGamefromSlot "SaveGameObject"))
              (bind _output_get_3 (Variables|Default|SetSaverSubClass _returnvalue_6))
              (bind _assave_game_object_3 (Utilities|Casting|CastToSaveGameObject _output_get_3))
              (Variables|/Game/ProgramBluePrint/PlayerObjective/SaveObjective/SaveGameObject.SaveGameObject_C|SetPlayerObjective _assave_game_object_3 "Go To FTI")
              (SaveGame|SaveGametoSlot (Variables|Default|GetSaverSubClass) "SaveGameObject")
              (else
                (bind _returnvalue_7 (SaveGame|CreateSaveGameObject "/Game/ProgramBluePrint/PlayerObjective/SaveObjective/SaveGameObject.SaveGameObject_C"))
                (bind _output_get_4 (Variables|Default|SetSaverSubClass _returnvalue_7))
                (bind _assave_game_object_4 (Utilities|Casting|CastToSaveGameObject _output_get_4))
                (Variables|/Game/ProgramBluePrint/PlayerObjective/SaveObjective/SaveGameObject.SaveGameObject_C|SetPlayerObjective _assave_game_object_4 "Go To FTI")
                (SaveGame|SaveGametoSlot (Variables|Default|GetSaverSubClass) "SaveGameObject"))))))
      (elif (== (Variables|/Game/ProgramBluePrint/Player/Player/ThirdPersonCharacter.ThirdPersonCharacter_C|GetSlot2Item _asthird_person_character) 0)
        (Variables|/Game/ProgramBluePrint/Player/Player/ThirdPersonCharacter.ThirdPersonCharacter_C|SetSlot2Item _asthird_person_character 1)
        (goto _label)
        (elif (== (Variables|/Game/ProgramBluePrint/Player/Player/ThirdPersonCharacter.ThirdPersonCharacter_C|GetSlot3Item _asthird_person_character) 0)
          (Variables|/Game/ProgramBluePrint/Player/Player/ThirdPersonCharacter.ThirdPersonCharacter_C|SetSlot3Item _asthird_person_character 1)
          (goto _label)
          (elif (== (Variables|/Game/ProgramBluePrint/Player/Player/ThirdPersonCharacter.ThirdPersonCharacter_C|GetSlot4Item _asthird_person_character) 0)
            (Variables|/Game/ProgramBluePrint/Player/Player/ThirdPersonCharacter.ThirdPersonCharacter_C|SetSlot4Item _asthird_person_character 1)
            (goto _label)
            (elif (== (Variables|/Game/ProgramBluePrint/Player/Player/ThirdPersonCharacter.ThirdPersonCharacter_C|GetSlot5Item _asthird_person_character) 0)
              (Variables|/Game/ProgramBluePrint/Player/Player/ThirdPersonCharacter.ThirdPersonCharacter_C|SetSlot5Item _asthird_person_character 1)
              (goto _label)
              (elif (== (Variables|/Game/ProgramBluePrint/Player/Player/ThirdPersonCharacter.ThirdPersonCharacter_C|GetSlotItem6 _asthird_person_character) 0)
                (Variables|/Game/ProgramBluePrint/Player/Player/ThirdPersonCharacter.ThirdPersonCharacter_C|SetSlotItem6 _asthird_person_character 1)
                (goto _label)
                (elif (== (Variables|/Game/ProgramBluePrint/Player/Player/ThirdPersonCharacter.ThirdPersonCharacter_C|GetSlotItem7 _asthird_person_character) 0)
                  (Variables|/Game/ProgramBluePrint/Player/Player/ThirdPersonCharacter.ThirdPersonCharacter_C|SetSlotItem7 _asthird_person_character 1)
                  (goto _label)
                  (elif (== (Variables|/Game/ProgramBluePrint/Player/Player/ThirdPersonCharacter.ThirdPersonCharacter_C|GetSlotItem8 _asthird_person_character) 0)
                    (Variables|/Game/ProgramBluePrint/Player/Player/ThirdPersonCharacter.ThirdPersonCharacter_C|SetSlotItem8 _asthird_person_character 1)
                    (goto _label)
                    (else
                      (bind _returnvalue_8 (UserInterface|CreateWidget "/Game/ProgramBluePrint/Inventory/Widget/InventoryFull.InventoryFull_C"))
                      (UserInterface|Viewport|AddtoViewport _returnvalue_8 0))))))))))))

(event EventBeginPlay
  (Utilities|FlowControl|Delay 3.0)
  (Variables|Default|SetCanPickUp true))

(fn ConstructionScript)