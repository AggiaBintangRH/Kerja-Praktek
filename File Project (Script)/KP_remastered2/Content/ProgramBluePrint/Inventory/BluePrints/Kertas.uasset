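; Kertas is a quest item pickup, apparently a test paper, that becomes collectible three seconds after BeginPlay.
; On box overlap it fills the character's first empty slot of eight with item 6, or shows an InventoryFull widget.
; On success it destroys itself, sets HasKey6, shows ObjectiveComplete and saves the "Talk To Dean" objective.
; Its save-existence check uses slot "Take A Test Paper", while loading and saving use "SaveGameObject".
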(event OnComponentBeginOverlap(Box)
  (params (OverlappedComponent :type Primitive%20Component%20Object%20Reference) (OtherActor :type Actor%20Object%20Reference) (OtherComp :type Primitive%20Component%20Object%20Reference) (OtherBodyIndex :type Integer) (bFromSweep :type Boolean) (SweepResult :type Hit%20Result%20Structure%20%28by%20ref%29))
  (if (Variables|Default|GetCanPickUp)
    (bind _asthird_person_character (Utilities|Casting|CastToThirdPersonCharacter (Game|GetPlayerCharacter 0)))
    (if (== (Variables|/Game/ProgramBluePrint/Player/Player/ThirdPersonCharacter.ThirdPersonCharacter_C|GetSlot1Item _asthird_person_character) 0)
      (Variables|/Game/ProgramBluePrint/Player/Player/ThirdPersonCharacter.ThirdPersonCharacter_C|SetSlot1Item _asthird_person_character 6)
      (Actor|DestroyActor :!label _label)
      (bind _asthird_person_character_2 (Utilities|Casting|CastToThirdPersonCharacter (Game|GetPlayerCharacter 0)))
      (Variables|/Game/ProgramBluePrint/Player/Player/ThirdPersonCharacter.ThirdPersonCharacter_C|SetHasKey6 _asthird_person_character_2 true)
      (bind _returnvalue (UserInterface|CreateWidget "/Game/ProgramBluePrint/PlayerObjective/Widget/ObjectiveComplete.ObjectiveComplete_C"))
      (UserInterface|Viewport|AddtoViewport _returnvalue 0)
      (bind _asthird_person_character_3 (Utilities|Casting|CastToThirdPersonCharacter (Game|GetPlayerCharacter 0)))
      (Variables|/Game/ProgramBluePrint/Player/Player/ThirdPersonCharacter.ThirdPersonCharacter_C|SetPlayerObjective _asthird_person_character_3 "Talk To Dean")
      (bind _returnvalue_2 (SaveGame|DoesSaveGameExist "Take A Test Paper"))
      (if _returnvalue_2
        (bind _returnvalue_3 (SaveGame|LoadGamefromSlot "SaveGameObject"))
        (bind _output_get (Variables|Default|SetSaverSubClass _returnvalue_3))
        (bind _assave_game_object (Utilities|Casting|CastToSaveGameObject _output_get))
        (Variables|/Game/ProgramBluePrint/PlayerObjective/SaveObjective/SaveGameObject.SaveGameObject_C|SetPlayerObjective _assave_game_object "Talk To Dean")
        (SaveGame|SaveGametoSlot (Variables|Default|GetSaverSubClass) "SaveGameObject")
        (else
          (bind _returnvalue_4 (SaveGame|CreateSaveGameObject "/Game/ProgramBluePrint/PlayerObjective/SaveObjective/SaveGameObject.SaveGameObject_C"))
          (bind _output_get_2 (Variables|Default|SetSaverSubClass _returnvalue_4))
          (bind _assave_game_object_2 (Utilities|Casting|CastToSaveGameObject _output_get_2))
          (Variables|/Game/ProgramBluePrint/PlayerObjective/SaveObjective/SaveGameObject.SaveGameObject_C|SetPlayerObjective _assave_game_object_2 "Talk To Dean")
          (SaveGame|SaveGametoSlot (Variables|Default|GetSaverSubClass) "SaveGameObject")))
      (elif (== (Variables|/Game/ProgramBluePrint/Player/Player/ThirdPersonCharacter.ThirdPersonCharacter_C|GetSlot2Item _asthird_person_character) 0)
        (Variables|/Game/ProgramBluePrint/Player/Player/ThirdPersonCharacter.ThirdPersonCharacter_C|SetSlot2Item _asthird_person_character 6)
        (goto _label)
        (elif (== (Variables|/Game/ProgramBluePrint/Player/Player/ThirdPersonCharacter.ThirdPersonCharacter_C|GetSlot3Item _asthird_person_character) 0)
          (Variables|/Game/ProgramBluePrint/Player/Player/ThirdPersonCharacter.ThirdPersonCharacter_C|SetSlot3Item _asthird_person_character 6)
          (goto _label)
          (elif (== (Variables|/Game/ProgramBluePrint/Player/Player/ThirdPersonCharacter.ThirdPersonCharacter_C|GetSlot4Item _asthird_person_character) 0)
            (Variables|/Game/ProgramBluePrint/Player/Player/ThirdPersonCharacter.ThirdPersonCharacter_C|SetSlot4Item _asthird_person_character 6)
            (goto _label)
            (elif (== (Variables|/Game/ProgramBluePrint/Player/Player/ThirdPersonCharacter.ThirdPersonCharacter_C|GetSlot5Item _asthird_person_character) 0)
              (Variables|/Game/ProgramBluePrint/Player/Player/ThirdPersonCharacter.ThirdPersonCharacter_C|SetSlot5Item _asthird_person_character 6)
              (goto _label)
              (elif (== (Variables|/Game/ProgramBluePrint/Player/Player/ThirdPersonCharacter.ThirdPersonCharacter_C|GetSlotItem6 _asthird_person_character) 0)
                (Variables|/Game/ProgramBluePrint/Player/Player/ThirdPersonCharacter.ThirdPersonCharacter_C|SetSlotItem6 _asthird_person_character 6)
                (goto _label)
                (elif (== (Variables|/Game/ProgramBluePrint/Player/Player/ThirdPersonCharacter.ThirdPersonCharacter_C|GetSlotItem7 _asthird_person_character) 0)
                  (Variables|/Game/ProgramBluePrint/Player/Player/ThirdPersonCharacter.ThirdPersonCharacter_C|SetSlotItem7 _asthird_person_character 6)
                  (goto _label)
                  (elif (== (Variables|/Game/ProgramBluePrint/Player/Player/ThirdPersonCharacter.ThirdPersonCharacter_C|GetSlotItem8 _asthird_person_character) 0)
                    (Variables|/Game/ProgramBluePrint/Player/Player/ThirdPersonCharacter.ThirdPersonCharacter_C|SetSlotItem8 _asthird_person_character 6)
                    (goto _label)
                    (else
                      (bind _returnvalue_5 (UserInterface|CreateWidget "/Game/ProgramBluePrint/Inventory/Widget/InventoryFull.InventoryFull_C"))
                      (UserInterface|Viewport|AddtoViewport _returnvalue_5 0))))))))))))

(event EventBeginPlay
  (Utilities|FlowControl|Delay 3.0)
  (Variables|Default|SetCanPickUp true))

(fn ConstructionScript)